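; BP_Door is a sliding double door that opens while the first player pawn is inside its Trigger and closes when it leaves.
; Overlap events move DoorL and DoorR apart or together one unit per step along their right vectors, with DoorNum counting steps to bound travel.
; A custom WhileLoopWithDelay macro paces the motion without Tick, and the shared IsOpen flag stops the opposing loop when direction reverses.
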(event OnComponentBeginOverlap(Trigger)
  (params (OverlappedComponent :type Primitive%20Component%20Object%20Reference) (OtherActor :type Actor%20Object%20Reference) (OtherComp :type Primitive%20Component%20Object%20Reference) (OtherBodyIndex :type Integer) (bFromSweep :type Boolean) (SweepResult :type Hit%20Result%20Structure%20%28by%20ref%29))
  (bind _doorl (Variables|Default|GetDoorL))
  (bind _doorr (Variables|Default|GetDoorR))
  (if (== OtherActor (Game|Player|GetPlayerPawn 0))
    (Utilities|FlowControl|Sequence
      (:then_0
        (Variables|Default|SetIsOpen false))
      (:then_1
        (Utilities|WhileLoopwithDelay 0.02 (and (not (Variables|Default|GetIsOpen)) (<= (Variables|Default|GetDoorNum) 101))
          (:Loop%20Body
            (Utilities|FlowControl|Sequence
              (:then_0
                (Transformation|SetWorldLocation _doorl (+ (* (Math|Vector|GetRightVector _doorl) -1) (Transformation|GetWorldLocation _doorl)) false false))
              (:then_1
                (Transformation|SetWorldLocation _doorr (+ (* (Math|Vector|GetRightVector _doorr) 1) (Transformation|GetWorldLocation _doorr)) false false))
              (:then_2
                (Variables|Default|SetDoorNum (+ (Variables|Default|GetDoorNum) 1)))))
          (:Completed
            (Variables|Default|SetIsOpen true)))))))

(event OnComponentEndOverlap(Trigger)
  (params (OverlappedComponent :type Primitive%20Component%20Object%20Reference) (OtherActor :type Actor%20Object%20Reference) (OtherComp :type Primitive%20Component%20Object%20Reference) (OtherBodyIndex :type Integer))
  (bind _doorl (Variables|Default|GetDoorL))
  (bind _doorr (Variables|Default|GetDoorR))
  (if (== OtherActor (Game|Player|GetPlayerPawn 0))
    (Utilities|FlowControl|Sequence
      (:then_0
        (Variables|Default|SetIsOpen true))
      (:then_1
        (Utilities|WhileLoopwithDelay 0.02 (and (Variables|Default|GetIsOpen) (> (Variables|Default|GetDoorNum) 0))
          (:Loop%20Body
            (Utilities|FlowControl|Sequence
              (:then_0
                (Transformation|SetWorldLocation _doorl (+ (* (Math|Vector|GetRightVector _doorl) 1) (Transformation|GetWorldLocation _doorl)) false false))
              (:then_1
                (Transformation|SetWorldLocation _doorr (+ (* (Math|Vector|GetRightVector _doorr) -1) (Transformation|GetWorldLocation _doorr)) false false))
              (:then_2
                (bind _result (Math|Integer|DecrementInt (Variables|Default|GetDoorNum))
                  (:%20%20
                    (Variables|Default|SetDoorNum _result))))))
          (:Completed
            (Variables|Default|SetIsOpen false)))))))

(fn ConstructionScript)