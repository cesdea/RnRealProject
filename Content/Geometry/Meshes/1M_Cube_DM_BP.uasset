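; A destructible cube actor that breaks after taking repeated hits from FirstPersonProjectile.
; Component hits from that projectile increment the float IsBreak, which acts as a hit counter despite its name.
; Once the counter reaches the threshold, the next hit enables physics on the Destructible component and applies small-radius radial damage at the impact point.
; The actor destroys itself after a short delay.
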(event OnComponentHit(Destructible)
  (params (HitComponent :type Primitive%20Component%20Object%20Reference) (OtherActor :type Actor%20Object%20Reference) (OtherComp :type Primitive%20Component%20Object%20Reference) (NormalImpulse :type Vector :default "0, 0, 0") (Hit :type Hit%20Result%20Structure%20%28by%20ref%29))
  (bind _asfirst_person_projectile (Utilities|Casting|CastToFirstPersonProjectile OtherActor))
  (if (>= (Variables|Default|GetIsBreak) 5.0)
    (Physics|SetSimulatePhysics (Variables|Default|GetDestructible) true)
    (Game|Damage|ApplyRadialDamage 1e+02 (.ImpactPoint (Collision|BreakHitResult Hit)) 1e+01 0 0 _asfirst_person_projectile 0 false "ECC_Visibility")
    (Utilities|FlowControl|Delay 2.0)
    (Actor|DestroyActor)
    (else
      (Variables|Default|SetIsBreak (+ (Variables|Default|GetIsBreak) 1.0)))))

(event EventBeginPlay)

(event Collision|EventActorBeginOverlap
  (params (OtherActor :type Actor%20Object%20Reference)))

(event EventTick
  (params (DeltaSeconds :type Float%20%28single-precision%29)))

(fn ConstructionScript)